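; Projectile that teleports its owner or scores a goal, flying a manually computed ballistic arc from launch speed, angle, gravity and elapsed time.
; Tick sets its position from the launch point, along its flattened forward vector and the owner's up vector.
; Overlapping a "Teleport" actor rotates the owner's up away from that actor, then moves the owner to the impact point.
; A "GoalCollider" component destroys its actor and prints "Goal!"; either hit destroys the projectile.
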(event OnComponentBeginOverlap(StaticMesh)
  (params (OverlappedComponent :type Primitive%20Component%20Object%20Reference) (OtherActor :type Actor%20Object%20Reference) (OtherComp :type Primitive%20Component%20Object%20Reference) (OtherBodyIndex :type Integer) (bFromSweep :type Boolean) (SweepResult :type Hit%20Result%20Structure%20%28by%20ref%29))
  (bind _returnvalue (Components|GetOwner))
  (if (Actor|ActorHasTag OtherActor "Teleport")
    (Transformation|SetActorRotation _returnvalue (Math|Rotator|MakeRotfromZ (- (Transformation|GetActorLocation (Components|GetOwner)) (Transformation|GetActorLocation OtherActor))))
    (Transformation|SetActorLocation _returnvalue (Transformation|GetActorLocation) false false)
    (Actor|DestroyActor)
    (elif (Components|ComponentHasTag OtherComp "GoalCollider")
      (Actor|DestroyActor OtherActor)
      (Development|PrintString "Goal!")
      (Actor|DestroyActor))))

(event Custom|Fire
  (params (LaunchSpeed :type Float%20%28single-precision%29) (LaunchAngle :type Float%20%28single-precision%29))
  (Variables|Default|SetLaunchSpeed LaunchSpeed)
  (Variables|Default|SetLaunchAngle LaunchAngle))

(event EventBeginPlay
  (Variables|Default|SetLaunchPosition (Transformation|GetActorLocation)))

(event EventTick
  (params (DeltaSeconds :type Float%20%28single-precision%29))
  (bind _returnvalue (Transformation|GetActorForwardVector))
  (Variables|Default|SetTime (+ DeltaSeconds (Variables|Default|GetTime)))
  (Transformation|SetActorLocation (+ (* (Math|Vector|Normalize (Math|Vector|MakeVector (.x _returnvalue) (.y _returnvalue) 0.0)) (CallFunction|GetDisplacementX)) (* (Transformation|GetActorUpVector (Components|GetOwner)) (CallFunction|GetDisplacementY)) (Variables|Default|GetLaunchPosition)) false false))

(fn ConstructionScript)

(fn GetDisplacementX
  (return (* (Variables|Default|GetLaunchSpeed) (Variables|Default|GetTime) (Math|Trig|Cos(Degrees) (Variables|Default|GetLaunchAngle)))))

(fn GetDisplacementY
  (return (- (* (Variables|Default|GetLaunchSpeed) (Variables|Default|GetTime) (Math|Trig|Sin(Degrees) (Variables|Default|GetLaunchAngle))) (/ (* (Variables|Default|GetGravity) (Math|Float|Power (Variables|Default|GetTime) 2.0)) 2.0))))