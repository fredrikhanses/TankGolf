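; BP_Tank is a player-controlled tank that drives along its forward vector and aims independently of the hull.
; MoveForward feeds movement input, while Turn yaws the whole actor, flipping the steering direction when the forward axis is negative so reversing steers inverted.
; TurnMouse adds yaw to the Head component and LookUp adds pitch to the SpringArm, with no clamping on either.
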(event Input|AxisEvents|InputAxisMoveForward
  (params (AxisValue :type Float%20%28single-precision%29))
  (Pawn|Input|AddMovementInput (Transformation|GetActorForwardVector) AxisValue false))

(event Input|AxisEvents|InputAxisTurn
  (params (AxisValue :type Float%20%28single-precision%29))
  (Transformation|SetActorRotation (Math|Rotator|CombineRotators (Math|Rotator|MakeRotator 0.0 0.0 (* AxisValue (+ (* (Math|Conversions|ToFloat(Boolean) (< (Input|AxisValues|GetMoveForward) 0.0)) -2.0) 1.0))) (Transformation|GetActorRotation))))

(event Input|AxisEvents|InputAxisTurnMouse
  (params (AxisValue :type Float%20%28single-precision%29))
  (Transformation|SetRelativeRotation (Variables|Default|GetHead) (Math|Rotator|MakeRotator 0.0 0.0 (+ AxisValue (.yaw (Variables|/Script/Engine.SceneComponent|GetRelativeRotation (Variables|Default|GetHead))))) false false))

(event Input|AxisEvents|InputAxisLookUp
  (params (AxisValue :type Float%20%28single-precision%29))
  (Transformation|SetRelativeRotation (Variables|Default|GetSpringArm) (Math|Rotator|MakeRotator 0.0 (+ AxisValue (.pitch (Variables|/Script/Engine.SceneComponent|GetRelativeRotation (Variables|Default|GetSpringArm)))) 0.0) false false))

(fn ConstructionScript)