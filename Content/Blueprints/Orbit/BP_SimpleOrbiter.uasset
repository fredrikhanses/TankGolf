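; Orbiter actor that moves its Planet component along an elliptical orbit with a smaller, tilted elliptical orbit layered on top.
; Each Tick, OrbitSolver derives positions from game time, rate and offset, stretches them on Y and sums both orbits.
; DrawOrbit passes positions through while leaving red and yellow debug-point trails, with optional circle drawing.
; The construction script previews the starting position from Radius and Offset, without the stretch or secondary orbit.
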(event EventTick
  (params (DeltaSeconds :type Float%20%28single-precision%29))
  (bind (_returnlocation _returnradius) (CallFunction|OrbitSolver 1e+02 0.0 2e+02))
  (bind _rate (Variables|Default|GetRate))
  (bind _radius (Variables|Default|GetRadius))
  (bind _offset (Variables|Default|GetOffset))
  (bind (_returnlocation_2 _returnradius_2) (CallFunction|OrbitSolver _radius _offset _rate))
  (bind _returnvalue (* _returnlocation_2 "1.000000,1.500000,1.000000"))
  (bind _returnlocation_3 (CallFunction|DrawOrbit _returnvalue "(R=1.000000,G=0.000000,B=0.000000,A=1.000000)" _returnradius_2 false "0, 0, 0"))
  (Transformation|SetRelativeLocation (Variables|Default|GetPlanet) (CallFunction|DrawOrbit (+ _returnlocation_3 (Math|Vector|RotateVector (* _returnlocation "1.000000,1.500000,1.000000") "0, 0,45.000000")) "(R=1.000000,G=1.000000,B=0.000000,A=1.000000)" _returnradius false _returnlocation_3) false false))

(fn ConstructionScript
  (Transformation|SetRelativeLocation (Variables|Default|GetPlanet) (Math|Vector|RotateVector (Math|Vector|MakeVector (Variables|Default|GetRadius) 0.0 0.0) (Math|Rotator|MakeRotator 0.0 0.0 (Math|Float|Absolute(Float) (Math|Float|%(Float) (Variables|Default|GetOffset) 3.6e+02)))) false false))

(fn OrbitSolver
  (params (Radius :type Float%20%28single-precision%29) (Offset :type Float%20%28single-precision%29) (Rate :type Float%20%28single-precision%29))
  (return (Math|Vector|RotateVector (Math|Vector|MakeVector Radius 0.0 0.0) (Math|Rotator|MakeRotator 0.0 0.0 (Math|Float|Absolute(Float) (Math|Float|%(Float) (+ Offset (* Rate (Utilities|Time|GetGameTimeinSeconds))) 3.6e+02)))) Radius))

(fn DrawOrbit
  (params (Position :type Vector) (PointColor :type Linear%20Color%20Structure) (Radius :type Float%20%28single-precision%29) (bDrawCircle :type Boolean) (ParentOrbit :type Vector))
  (Rendering|Debug|DrawDebugPoint (+ Position (Transformation|GetActorLocation)) 2.0 PointColor 15.0)
  (if bDrawCircle
    (Rendering|Debug|DrawDebugCircle (+ ParentOrbit (Transformation|GetActorLocation)) Radius 64 PointColor 0.0 2.0 "1.000000,0.000000,0.000000" "0.000000,1.000000,0.000000"))
  (return Position))